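; BP_Arrow is a physics-driven arrow projectile, filed under dangers, that launches itself forward with a velocity-change impulse on BeginPlay.
; Tick counts down a lifetime timer and destroys the actor when it expires.
; The first hit clears Alive, ignores the Pawn channel, enables gravity and adds random upward impulse and torque, so the spent arrow tumbles briefly before being destroyed.
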(event OnComponentHit(Arrow)
  (params (HitComponent :type Primitive%20Component%20Object%20Reference) (OtherActor :type Actor%20Object%20Reference) (OtherComp :type Primitive%20Component%20Object%20Reference) (NormalImpulse :type Vector :default "0, 0, 0") (Hit :type Hit%20Result%20Structure%20%28by%20ref%29))
  (bind _arrow (Variables|Default|GetArrow))
  (Utilities|FlowControl|DoOnce false
    (:Completed
      (Variables|Default|SetAlive false)
      (Collision|SetCollisionResponsetoChannel (Variables|Default|GetArrow) "ECC_Pawn" "ECR_Ignore")
      (Physics|SetEnableGravity _arrow true)
      (Physics|AddImpulse (Variables|Default|GetArrow) (* (Math|Vector|GetUpVector _arrow) (+ (* (Math|Random|RandomFloat) 5e+01) 5e+01)) "None" false)
      (Class|PrimitiveComponent|AddTorqueinDegrees (Variables|Default|GetArrow) (Math|Vector|MakeVector (- (* (Math|Random|RandomFloat) 9e+03) 4.5e+03) (- (* (Math|Random|RandomFloat) 9e+03) 4.5e+03) (- (* (Math|Random|RandomFloat) 9e+03) 4.5e+03)) "None" true)
      (Variables|Default|SetLifetimeTimer (+ (Variables|Default|GetLifetimeTimer) 1.5))
      (Utilities|FlowControl|Delay 1.5)
      (Actor|DestroyActor))))

(event EventBeginPlay
  (Physics|AddImpulse (Variables|Default|GetArrow) (* (Math|Vector|GetForwardVector (Variables|Default|GetArrow)) 1e+03) "None" true))

(event EventTick
  (params (DeltaSeconds :type Float%20%28single-precision%29))
  (Variables|Default|SetLifetimeTimer (- (Variables|Default|GetLifetimeTimer) DeltaSeconds))
  (if (<= (Variables|Default|GetLifetimeTimer) 0.0)
    (Actor|DestroyActor)))

(fn ConstructionScript)