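; BP_ArrowShooter is a danger actor that continually fires BP_Arrow projectiles from its ShootArea component.
; Tick feeds a Delay with a clamped random duration, which acts as a repeating, irregular fire timer.
; Each arrow takes the area's rotation and world X, with random world Y and Z within half its bounds extent around the center.
; Spawning ignores collisions, so every shot produces an arrow.
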(event EventBeginPlay)

(event Collision|EventActorBeginOverlap
  (params (OtherActor :type Actor%20Object%20Reference)))

(event EventTick
  (params (DeltaSeconds :type Float%20%28single-precision%29))
  (bind _shootarea (Variables|Default|GetShootArea))
  (bind _boxextent (Collision|GetComponentBounds _shootarea))
  (bind _returnvalue (Transformation|GetWorldLocation _shootarea))
  (bind _returnvalue_2 (/ (.z _boxextent) 2.0))
  (bind _returnvalue_3 (/ (.y _boxextent) 2.0))
  (Utilities|FlowControl|Delay (Math|Float|Clamp(Float) (+ (Math|Random|RandomFloat) 0.5) 0.7 1.5))
  (Game|SpawnActorfromClass "/Game/MyGame/Dangers/Projectiles/BP_Arrow.BP_Arrow_C" (Math|Transform|MakeTransform (Math|Vector|MakeVector (.x _returnvalue) (Math|Random|RandomFloatinRange (- (.y _returnvalue) _returnvalue_3) (+ (.y _returnvalue) _returnvalue_3)) (Math|Random|RandomFloatinRange (- (.z _returnvalue) _returnvalue_2) (+ (.z _returnvalue) _returnvalue_2))) (Transformation|GetWorldRotation _shootarea) "1.000000,1.000000,1.000000") "AlwaysSpawn" "MultiplyWithRoot" 0 0))

(fn ConstructionScript)